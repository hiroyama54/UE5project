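; Paper2D player pawn with Enhanced Input movement and two-state flipbook animation.
; BeginPlay adds the IMC_RPG mapping context, and IA_Move feeds movement input along world forward and right axes.
; Each tick picks the running or idle flipbook from speed, then flips control yaw between 0 and 180 by X velocity sign.
; At zero X velocity, facing follows BisMovingRight, which these graphs never set.
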(event `UpdateAnimation`
  ;[1 1 1] Handle Animation
  (`PaperFlipbookComponent.SetFlipbook` (`self.Sprite`) (select `bool` (> (`KismetMathLibrary.VSize` (`self.GetVelocity`)) 0.0) :`false` "/Game/Paper2D/Content/2DSideScroller/Sprites/IdleAnimation.IdleAnimation" :`true` "/Game/Paper2D/Content/2DSideScroller/Sprites/RunningAnimation.RunningAnimation" :!type "PaperFlipbook Object Reference")))

(event `self.ReceiveBeginPlay`
  (`parent.ReceiveBeginPlay`)
  (bind _asplayer_controller (cast `PlayerController` (`GameplayStatics.GetPlayerController` 0)))
  (message `EnhancedInputSubsystemInterface.AddMappingContext` (pcsubsystem `EnhancedInputLocalPlayerSubsystem` _asplayer_controller) "/Game/Paper2D/MyContent/Input/InputMappingContext/IMC_RPG.IMC_RPG" 0 (struct)))

(event `self.ReceiveTick`
  (params (DeltaSeconds :type "Float (single-precision)"))
  (bind _returnvalue (`self.GetController`))
  (bind _returnvalue_2 (`self.GetController`))
  ;[1 1 1] Tick - Updates animation
  (`parent.ReceiveTick` DeltaSeconds)
  (`self.UpdateAnimation`)
  (`/Engine/EditorBlueprintResources/StandardMacros.CompareFloat` (.x (`MovementComponent.Velocity` (`self.GetMovementComponent`)))
    (:`>`
      (`/Engine/EditorBlueprintResources/StandardMacros.IsValid` _returnvalue_2 :!label _label
        (:`Is Valid`
          (`Controller.SetControlRotation` _returnvalue_2 (`KismetMathLibrary.MakeRotator` 0.0)))))
    (:`==`
      (if (`self.bisMovingRight`)
        (goto _label)
        (else
          (`/Engine/EditorBlueprintResources/StandardMacros.IsValid` _returnvalue :!label _label_2
            (:`Is Valid`
              (`Controller.SetControlRotation` _returnvalue (`KismetMathLibrary.MakeRotator` 0.0 0.0 180.0)))))))
    (:`<`
      (goto _label_2))))

(event `EnhancedInput|/Game/Paper2D/MyContent/Input/InputAction/IA_Move`
  (params (ActionValue :type "Vector2D Structure") (ElapsedSeconds :type "Float (double-precision)") (TriggeredSeconds :type "Float (double-precision)") (InputAction :type "InputAction Object Reference" :default "/Game/Paper2D/MyContent/Input/InputAction/IA_Move.IA_Move"))
  (bind (_x _y) (`KismetMathLibrary.BreakVector2D` ActionValue))
  (:`Triggered`
    (`self.AddMovementInput` (`KismetMathLibrary.Vector_Forward`) _x)
    (`self.AddMovementInput` (`KismetMathLibrary.Vector_Right`) _y)))

(fn `UserConstructionScript`
  (`parent.UserConstructionScript`))